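; Moving platform actor that shuttles continuously between StartLocation and EndLocation from BeginPlay.
; A Timeline's MovementPath track drives a vector lerp that sets the actor's location without sweeping.
; When the Timeline finishes, its direction selects reverse or forward playback, creating an endless ping-pong.
; Play rate is TotalTime divided by 60, so a larger TotalTime makes the platform move faster.
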(event Custom|MovePlatformToStartLocation
  (Components|Timeline|SetPlayRate (Variables|Default|GetTimeline) (/ (Variables|Default|GetTotalTime) 6e+01))
  (bind (_direction _movementpath) (Timeline|Timeline ReverseFromEnd)
    (:Update
      (Transformation|SetActorLocation (Math|Vector|Lerp(Vector) (Variables|Default|GetStartLocation) (Variables|Default|GetEndLocation) _movementpath) false false))
    (:Finished
      (switch Utilities|FlowControl|Switch|SwitchonETimelineDirection _direction
        (:Forward
          (CallFunction|MovePlatformtoStartLocation))
        (:Backward
          (CallFunction|MovePlatformtoEndLocation))))))

(event Custom|MovePlatformToEndLocation
  (Components|Timeline|SetPlayRate (Variables|Default|GetTimeline) (/ (Variables|Default|GetTotalTime) 6e+01))
  (bind (_direction _movementpath) (Timeline|Timeline PlayFromStart)
    (:Update
      (Transformation|SetActorLocation (Math|Vector|Lerp(Vector) (Variables|Default|GetStartLocation) (Variables|Default|GetEndLocation) _movementpath) false false))
    (:Finished
      (switch Utilities|FlowControl|Switch|SwitchonETimelineDirection _direction
        (:Forward
          (CallFunction|MovePlatformtoStartLocation))
        (:Backward
          (CallFunction|MovePlatformtoEndLocation))))))

(event EventBeginPlay
  (CallFunction|MovePlatformtoEndLocation))

(event Collision|EventActorBeginOverlap
  (params (OtherActor :type Actor%20Object%20Reference)))

(event EventTick
  (params (DeltaSeconds :type Float%20%28single-precision%29)))

(fn ConstructionScript)